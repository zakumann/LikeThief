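; Player character Blueprint with a work-in-progress, mesh-free footstep system driven from Tick.
; While the character is not falling and horizontal speed is below a small threshold, it plays a footstep cue and reports a "Footstep" noise event every frame.
; FootstepTimer does not accumulate; it takes DeltaSeconds, serves as the volume multiplier, then resets.
; The crouch input event is empty, and its FlipFlop, Crouch and UnCrouch nodes are unconnected.
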(event `self.ReceiveTick`
  (params (DeltaSeconds :type "Float (single-precision)"))
  (bind _returnvalue (`self.K2_GetActorLocation`))
  ; Footstep-SoundFX(NoMesh)
  (if (or false false (`NavMovementInterface.IsFalling` (`self.CharacterMovement`)))
    (set `self.FootstepTimer` 0.0)
    (elif (< (`KismetMathLibrary.VSizeXY` (`self.GetVelocity`)) 10.0)
      ;; Connect with delta seconds
      (bind _output_get (set `self.FootstepTimer` DeltaSeconds))
      (`GameplayStatics.PlaySoundAtLocation` "/Game/SoundEffects/SFX_FootstepCue.SFX_FootstepCue" _returnvalue (struct) _output_get 1.0 0.0 null null null null)
      (`AISense_Hearing.ReportNoiseEvent` _returnvalue 0.2 self 1000.0 "Footstep")
      (set `self.FootstepTimer` 0.0))))

(event `EnhancedInput|/Game/Input/Actions/IA_Crouch`
  (params (ActionValue :type Boolean) (ElapsedSeconds :type "Float (double-precision)") (TriggeredSeconds :type "Float (double-precision)") (InputAction :type "InputAction Object Reference" :default "/Game/Input/Actions/IA_Crouch.IA_Crouch")))

(fn `UserConstructionScript`)