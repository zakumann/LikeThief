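; AI controller for enemies that runs the enemy behavior tree on BeginPlay and reports sight of the player.
; Perception updates for the player character broadcast a sight-registered dispatcher with the sensed state and a detection speed.
; That speed comes from a float curve sampled by the normalized distance between stimulus and receiver.
; SeenPlayer only prints a debug string, and LostPlayer is an empty stub.
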(event `self.ReceiveBeginPlay`
  (`self.RunBehaviorTree` "/Game/Blueprint/AI/BT_Enemy.BT_Enemy"))

(event `self.AIPerception.OnTargetPerceptionUpdated`
  (params (Actor :type "Actor Object Reference") (Stimulus :type "AIStimulus Structure"))
  (bind (_age _expirationage _strength _stimuluslocation _receiverlocation _tag _bsuccessfullysensed) (break `AIStimulus` Stimulus))
  (if (== Actor (`GameplayStatics.GetPlayerCharacter` 0))
    (`self.SightRegisteredED` _bsuccessfullysensed (`CurveFloat.GetFloatValue` (`self.SighrCurve`) (`KismetMathLibrary.NormalizeToRange` (`KismetMathLibrary.Vector_Distance` _stimuluslocation _receiverlocation) 0.0 500.0)))))

(event `SeenPlayer`
  (`KismetSystemLibrary.PrintString` "Hello"))

(event `LostPlayer`)

(fn `UserConstructionScript`)