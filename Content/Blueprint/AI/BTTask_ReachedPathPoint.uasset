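; Behavior tree task that advances an enemy guard's patrol index when it reaches a path point.
; It casts the controlled pawn to BP_EnemyGuard and steps CurrentPathIndex by PathDirection while that index is valid in PatrolPath.
; At the path's end, PatrolPathBehavior decides whether the guard stays put, reverses direction or loops to the first point.
; Each of these branches finishes the task successfully.
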(event `self.ReceiveExecuteAI`
  (params (OwnerController :type "AIController Object Reference") (ControlledPawn :type "Pawn Object Reference"))
  (bind _guardenemypawn (`self.GuardEnemyPawn`))
  (bind _guardenemypawn_2 (`self.GuardEnemyPawn`))
  (bind _asbp_enemy_guard (cast `/Game/Blueprint/AI/BP_EnemyGuard` ControlledPawn))
  (bind _output_get (set `self.GuardEnemyPawn` _asbp_enemy_guard))
  (if (`KismetArrayLibrary.Array_IsValidIndex` (`EnemyGuard.PatrolPath` _output_get) (+ (`EnemyGuard.CurrentPathIndex` _output_get) (`/Game/Blueprint/AI/BP_EnemyGuard.PathDirection` _output_get)))
    (set `EnemyGuard.CurrentPathIndex` (+ (`EnemyGuard.CurrentPathIndex` _guardenemypawn) (`/Game/Blueprint/AI/BP_EnemyGuard.PathDirection` _guardenemypawn)) _guardenemypawn)
    (`self.FinishExecute` true)
    (else
      (switch `EPatrolPathEnding` (`EnemyGuard.PatrolPathBehavior` (`self.GuardEnemyPawn`))
        (:`DoNothing`
          (`self.FinishExecute` true))
        (:`PatrolBack`
          (set `/Game/Blueprint/AI/BP_EnemyGuard.PathDirection` (* (`/Game/Blueprint/AI/BP_EnemyGuard.PathDirection` _guardenemypawn_2) -1) _guardenemypawn_2)
          (`self.FinishExecute` true))
        (:`Loop`
          (set `EnemyGuard.CurrentPathIndex` 0 (`self.GuardEnemyPawn`))
          (`self.FinishExecute` true))))))