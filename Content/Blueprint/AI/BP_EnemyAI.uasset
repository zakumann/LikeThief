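; Enemy AI controller that runs the BT_Enemy behavior tree and feeds its blackboard from sight and hearing perception.
; Perception updates go to HandleSense, which branches on the sense class's display name and sets IsInvestigating from the sensed state.
; Seeing the player sets the target actor and raises walk speed, with no reset here.
; Lost sight clears the actor and stores the stimulus location; hearing stores location only.
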(event `self.ReceiveBeginPlay`
  (`self.RunBehaviorTree` "/Game/Blueprint/AI/BT_Enemy.BT_Enemy"))

(event `self.AIPerception.OnTargetPerceptionUpdated`
  (params (Actor :type "Actor Object Reference") (Stimulus :type "AIStimulus Structure"))
  (bind _returnvalue (`AIPerceptionSystem.GetSenseClassForStimulus` Stimulus))
  (`self.HandleSense` (`KismetSystemLibrary.GetClassDisplayName` _returnvalue) Actor Stimulus))

(fn `HandleSense`
  (params (Selection :type String) (SensedActor :type "Actor Object Reference") (Stimulus :type "AIStimulus Structure"))
  (bind (_stimulus_age _stimulus_expirationage _stimulus_strength _stimulus_stimuluslocation) (break `AIStimulus` (`local.Stimulus`)))
  (bind (_stimulus_age_2 _stimulus_expirationage_2 _stimulus_strength_2 _stimulus_stimuluslocation_2 _stimulus_receiverlocation _stimulus_tag _stimulus_bsuccessfullysensed) (break `AIStimulus` (`local.Stimulus`)))
  (bind (_stimulus_age_3 _stimulus_expirationage_3 _stimulus_strength_3 _stimulus_stimuluslocation_3 _stimulus_receiverlocation_2 _stimulus_tag_2 _stimulus_bsuccessfullysensed_2) (break `AIStimulus` (`local.Stimulus`)))
  (bind (_stimulus_age_4 _stimulus_expirationage_4 _stimulus_strength_4 _stimulus_stimuluslocation_4) (break `AIStimulus` (`local.Stimulus`)))
  (switch `string` Selection
    (:`AISense_Sight`
      (`BlackboardComponent.SetValueAsBool` (`self.Blackboard`) "IsInvestigating" _stimulus_bsuccessfullysensed)
      (if _stimulus_bsuccessfullysensed
        ; Alert
        (if (== (`local.SensedActor`) (`GameplayStatics.GetPlayerCharacter` 0))
          (`BlackboardComponent.SetValueAsObject` (`self.Blackboard`) "TargetLocationActor" (`local.SensedActor`))
          (bind _ascharacter (cast `Character` (`self.K2_GetPawn`)))
          (set `CharacterMovementComponent.MaxWalkSpeed` 400.0 (`Character.CharacterMovement` _ascharacter)))
        (else
          (`BlackboardComponent.SetValueAsVector` (`self.Blackboard`) "TargetLocationVector" _stimulus_stimuluslocation_4)
          (`BlackboardComponent.SetValueAsObject` (`self.Blackboard`) "TargetLocationActor" null))))
    (:`AISense_Hearing`
      (`BlackboardComponent.SetValueAsBool` (`self.Blackboard`) "IsInvestigating" _stimulus_bsuccessfullysensed_2)
      (`BlackboardComponent.SetValueAsVector` (`self.Blackboard`) "TargetLocationVector" _stimulus_stimuluslocation))))

(fn `UserConstructionScript`)