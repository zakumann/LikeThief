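; Behavior tree task that sets up the next patrol move for a BP_EnemyGuard.
; It reads the guard's current PatrolPath point and writes a random reachable location near it to the blackboard, plus a wait time randomized by that point's deviation.
; It also sets the guard to walk speed, clears the caution flag and finishes successfully, without changing the path index itself.
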(event `self.ReceiveExecuteAI`
  (params (OwnerController :type "AIController Object Reference") (ControlledPawn :type "Pawn Object Reference"))
  (bind _guardenemypawn (`self.GuardEnemyPawn`))
  (bind _output (`|GetArrayItem` (`EnemyGuard.PatrolPath` _guardenemypawn) (`EnemyGuard.CurrentPathIndex` _guardenemypawn)))
  (bind _waittime (`PathPoint.WaitTime` _output))
  (bind _waitdeviation (`PathPoint.WaitDeviation` _output))
  (bind _asbp_enemy_guard (cast `/Game/Blueprint/AI/BP_EnemyGuard` ControlledPawn))
  (bind _output_get (set `self.GuardEnemyPawn` _asbp_enemy_guard))
  (`BTFunctionLibrary.SetBlackboardValueAsVector` (`self.BB_TargetVector`) (`NavigationSystemV1.K2_GetRandomReachablePointInRadius` (`Actor.K2_GetActorLocation` (`|GetArrayItem` (`EnemyGuard.PatrolPath` _output_get) (`EnemyGuard.CurrentPathIndex` _output_get))) 20.0 null null))
  (`BTFunctionLibrary.SetBlackboardValueAsFloat` (`self.BB_WaitTime`) (`KismetMathLibrary.RandomFloatInRange` (- _waittime _waitdeviation) (+ _waittime _waitdeviation)))
  (set `CharacterMovementComponent.MaxWalkSpeed` (`self.WalkSpeed`) (`Character.CharacterMovement` (`self.GuardEnemyPawn`)))
  (`BTFunctionLibrary.SetBlackboardValueAsBool` (`self.BB_CautionState`))
  (`self.FinishExecute` true))