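; BP_Puddle is a noise-maker puddle that plays footstep splashes and can report noise to AI while the player overlaps it.
; Each Tick, if no splash sound is active, it spawns one at the player, with volume normalized from player speed and printed for debugging.
; Splashes above a volume threshold report a noise event at the puddle, instigated by the player, then stop and clear after a short delay.
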(event `self.ReceiveTick`
  (params (DeltaSeconds :type "Float (single-precision)"))
  (bind _returnvalue (`GameplayStatics.GetPlayerCharacter` 0))
  (bind _returnvalue_2 (`KismetMathLibrary.NormalizeToRange` (`KismetMathLibrary.VSize` (`self.GetVelocity` _returnvalue)) 200.0 600.0))
  (if (`self.IsOverlappingActor` _returnvalue)
    (`self.SoundInstance`
      (:`then`)
      (:`else`
        (`KismetSystemLibrary.PrintString` (`KismetStringLibrary.Conv_DoubleToString` _returnvalue_2))
        (bind _returnvalue_3 (`GameplayStatics.SpawnSoundAtLocation` "/Game/Blueprint/NoiseMaker/Sound/Cue_FootstepPuddle.Cue_FootstepPuddle" (`self.K2_GetActorLocation` (`GameplayStatics.GetPlayerCharacter` 0)) (struct) _returnvalue_2 1.0 0.0 null null))
        (bind _output_get (set `self.SoundInstance` _returnvalue_3))
        (if (> (`AudioComponent.VolumeMultiplier` _output_get) 0.8)
          (`AISense_Hearing.ReportNoiseEvent` (`self.K2_GetActorLocation`) 1.0 (`GameplayStatics.GetPlayerCharacter` 0))
          (`KismetSystemLibrary.Delay` 0.5)
          (`AudioComponent.Stop` (`self.SoundInstance`))
          (set `self.SoundInstance` null))))))

(fn `UserConstructionScript`)